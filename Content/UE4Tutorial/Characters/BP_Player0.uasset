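; BP_Player0 is a player character Blueprint that sets up the player's HUD and reacts to damage.
; On BeginPlay it creates a crosshair widget and a player health bar widget and adds both to the viewport.
; When the AttributeComponent reports a negative health change, it writes the current game time into the mesh materials' TimeToHit parameter, likely driving a hit-flash effect in the shader.
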(event `self.ReceiveBeginPlay`
  (bind _returnvalue (`|CreateWidget` "/Game/UE4Tutorial/UI/CrosshairWidget.CrosshairWidget_C"))
  (`UserWidget.AddToViewport` _returnvalue 0)
  (bind _returnvalue_2 (`|CreateWidget` "/Game/UE4Tutorial/UI/PlayerHealthBar.PlayerHealthBar_C"))
  (`UserWidget.AddToViewport` _returnvalue_2 0))

(event `self.AttributeComponent.OnHealthChanged`
  (params (InstigatorActor :type "Actor Object Reference") (OwningComp :type "SAttributeComponent Object Reference") (NewHealth :type "Float (single-precision)") (HealthMax :type "Float (single-precision)") (Delta :type "Float (single-precision)"))
  (bind _mesh (`self.Mesh`))
  (if (< Delta 0.0)
    (`/Engine/EditorBlueprintResources/StandardMacros.IsValid` _mesh
      (:`Is Valid`
        (`MeshComponent.SetScalarParameterValueOnMaterials` _mesh "TimeToHit" (`GameplayStatics.GetTimeSeconds`))))))

(fn `UserConstructionScript`)