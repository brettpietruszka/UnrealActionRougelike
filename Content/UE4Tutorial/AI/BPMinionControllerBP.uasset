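; BPMinionControllerBP is a minion AI controller Blueprint whose only active logic is on-screen debugging of where its pawn faces and focuses.
; Each Tick it draws two colored debug strings above the controlled pawn: the control rotation's forward vector and the controller's focal point.
; Each string lasts for the frame's delta time, so it refreshes continuously; BeginPlay and the construction script are empty.
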(event `self.ReceiveTick`
  (params (DeltaSeconds :type "Float (single-precision)"))
  (bind _returnvalue (`self.K2_GetPawn`))
  (bind _returnvalue_2 (`self.K2_GetActorLocation` _returnvalue))
  (`KismetSystemLibrary.DrawDebugString` (+ _returnvalue_2 (0.0 0.0 30.0)) (`KismetStringLibrary.Conv_VectorToString` (`KismetMathLibrary.GetForwardVector` (`Pawn.GetControlRotation` _returnvalue))) null (struct :`R` 1.0 :`G` 0.208059 :`B` 0.714602 :`A` 1.0) DeltaSeconds)
  (`KismetSystemLibrary.DrawDebugString` (+ _returnvalue_2 (0.0 0.0 70.0)) (`KismetStringLibrary.Conv_VectorToString` (`self.GetFocalPoint`)) null (struct :`G` 1.0 :`B` 0.921536 :`A` 1.0) DeltaSeconds))

(fn `UserConstructionScript`)